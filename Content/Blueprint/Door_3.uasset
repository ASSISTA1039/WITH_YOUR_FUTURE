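; Door actor that swings open or closed through a timeline-driven yaw rotation when its OPENDOOR event fires inside its trigger zone.
; Box overlap enables player input, and for a Car2 it also stores this door in the car's DOOR3 variable and opens a Gate node.
; The Gate lets OPENDOOR reach a FlipFlop that alternates playing and reversing the timeline, until any end overlap disables input and closes it.
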(event OnComponentBeginOverlap(Box)
  (params (OverlappedComponent :type Primitive%20Component%20Object%20Reference) (OtherActor :type Actor%20Object%20Reference) (OtherComp :type Primitive%20Component%20Object%20Reference) (OtherBodyIndex :type Integer) (bFromSweep :type Boolean) (SweepResult :type Hit%20Result%20Structure%20%28by%20ref%29))
  (Input|EnableInput (Game|GetPlayerController 0))
  (bind _ascar_2 (Utilities|Casting|CastToCar2 OtherActor))
  (Variables|/Game/Blueprint/Car2.Car2_C|SetDOOR3 _ascar_2 self)
  (Utilities|FlowControl|Gate true) ; enters at Open
)

(event OnComponentEndOverlap(Box)
  (params (OverlappedComponent :type Primitive%20Component%20Object%20Reference) (OtherActor :type Actor%20Object%20Reference) (OtherComp :type Primitive%20Component%20Object%20Reference) (OtherBodyIndex :type Integer))
  (Input|DisableInput (Game|GetPlayerController 0))
  (Utilities|FlowControl|Gate true) ; enters at Close
)

(event Custom|OPENDOOR
  (Utilities|FlowControl|Gate true
    (:Exit
      (Utilities|FlowControl|FlipFlop
        (:A
          (bind _新建轨道_0 (Timeline|open Play)
            (:Update
              (Transformation|SetRelativeRotation (Variables|Default|GetDoor) (Math|Rotator|MakeRotator 0.0 0.0 _新建轨道_0) false false))))
        (:B
          (Timeline|open Reverse))))))

(fn ConstructionScript)