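; Car1 is a possessable vehicle that the player character boards and leaves.
; Box overlap shows a text prompt, sets the character's Vehicle reference and opens a gate for the board event 上车.
; Boarding possesses the car, plays a timeline sliding the Car component, then after a delay enables physics on Can and attaches the collision-less character to Up.
; E detaches the character to Down and, after a view blend, repossesses it.
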(event OnComponentBeginOverlap(Box)
  (params (OverlappedComponent :type Primitive%20Component%20Object%20Reference) (OtherActor :type Actor%20Object%20Reference) (OtherComp :type Primitive%20Component%20Object%20Reference) (OtherBodyIndex :type Integer) (bFromSweep :type Boolean) (SweepResult :type Hit%20Result%20Structure%20%28by%20ref%29))
  (bind _up (Variables|Default|GetUp))
  (bind _returnvalue (Transformation|GetWorldTransform _up))
  (bind (_location _rotation) (Math|Transform|BreakTransform _returnvalue))
  (bind _asbp_player_character (Utilities|Casting|CastToBP_PlayerCharacter OtherActor))
  (Variables|/Game/Player/BP_PlayerCharacter.BP_PlayerCharacter_C|SetVehicle _asbp_player_character self)
  (Rendering|SetVisibility (Variables|Default|GetTextRender) true false)
  (Utilities|FlowControl|Gate true) ; enters at Open
)

(event OnComponentEndOverlap(Box)
  (params (OverlappedComponent :type Primitive%20Component%20Object%20Reference) (OtherActor :type Actor%20Object%20Reference) (OtherComp :type Primitive%20Component%20Object%20Reference) (OtherBodyIndex :type Integer))
  (bind _up (Variables|Default|GetUp))
  (bind _returnvalue (Transformation|GetWorldTransform _up))
  (bind (_location _rotation) (Math|Transform|BreakTransform _returnvalue))
  (bind _asbp_player_character (Utilities|Casting|CastToBP_PlayerCharacter OtherActor))
  (Variables|/Game/Player/BP_PlayerCharacter.BP_PlayerCharacter_C|SetVehicle _asbp_player_character 0)
  (Rendering|SetVisibility (Variables|Default|GetTextRender) false false)
  (Utilities|FlowControl|Gate true) ; enters at Close
)

(event Custom|上车
  (params (character :type Pawn%20Object%20Reference))
  (bind _up (Variables|Default|GetUp))
  (bind _returnvalue (Transformation|GetWorldTransform _up))
  (bind (_location _rotation) (Math|Transform|BreakTransform _returnvalue))
  (Utilities|FlowControl|Gate true
    (:Exit
      (Variables|Default|SetCharacterRef character)
      (Pawn|Possess (Game|GetPlayerController 0) self)
      (bind _新建轨道_0 (Timeline|时间轴 Play)
        (:Update
          (Transformation|SetRelativeLocation (Variables|Default|GetCar) (Math|Vector|MakeVector _新建轨道_0 0.0 0.0) false false)
          (Utilities|FlowControl|Delay 1.5)
          (Physics|SetSimulatePhysics (Variables|Default|GetCan) true)
          (Transformation|SetActorTransform (Variables|Default|GetCharacterRef) (Math|Transform|MakeTransform _location _rotation "1.000000,1.000000,1.000000"))
          (Collision|SetActorEnableCollision (Variables|Default|GetCharacterRef) false)
          (Transformation|AttachComponentToComponent (Variables|Default|GetCharacterRef) (Variables|Default|GetUp) "None" "KeepWorld" "KeepWorld" "KeepWorld" true))))))

(event Input|KeyboardEvents|E
  (params (Key :type Key%20Structure :default "None"))
  (bind _returnvalue (Game|GetPlayerController 0))
  (bind _characterref (Variables|Default|GetCharacterRef))
  (bind _down (Variables|Default|GetDown))
  (bind _returnvalue_2 (Transformation|GetWorldTransform _down))
  (bind (_location _rotation) (Math|Transform|BreakTransform _returnvalue_2))
  (:Pressed
    (Utilities|IsValid _characterref
      (:Is%20Valid
        (Transformation|DetachFromActor _characterref "KeepWorld" "KeepRelative" "KeepWorld")
        (Transformation|SetActorTransform _characterref (Math|Transform|MakeTransform _location _rotation "1.000000,1.000000,1.000000"))
        (Collision|SetActorEnableCollision (Variables|Default|GetCharacterRef) false)
        (Game|Player|SetViewTargetwithBlend _returnvalue 0 0.2 "VTBlend_Linear" 0.0 false)
        (Utilities|FlowControl|Delay 0.2)
        (Pawn|Possess _returnvalue (Variables|Default|GetCharacterRef))))))

(fn ConstructionScript)