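; Car Blueprint with a box trigger that detects the player character, apparently an unfinished enter-and-exit vehicle interaction.
; Begin overlap only casts to BP_PlayerCharacter, while end overlap clears that character's Vehicle reference and closes a gate.
; The gate's exit calls Possess on the first player controller with no pawn supplied, and nothing opens or enters the gate.
; Input toggling and prompt text visibility nodes are disconnected and never run.
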(event OnComponentBeginOverlap(Box)
  (params (OverlappedComponent :type Primitive%20Component%20Object%20Reference) (OtherActor :type Actor%20Object%20Reference) (OtherComp :type Primitive%20Component%20Object%20Reference) (OtherBodyIndex :type Integer) (bFromSweep :type Boolean) (SweepResult :type Hit%20Result%20Structure%20%28by%20ref%29))
  (Utilities|Casting|CastToBP_PlayerCharacter OtherActor))

(event OnComponentEndOverlap(Box)
  (params (OverlappedComponent :type Primitive%20Component%20Object%20Reference) (OtherActor :type Actor%20Object%20Reference) (OtherComp :type Primitive%20Component%20Object%20Reference) (OtherBodyIndex :type Integer))
  (bind _asbp_player_character (Utilities|Casting|CastToBP_PlayerCharacter OtherActor))
  (Variables|/Game/Player/BP_PlayerCharacter.BP_PlayerCharacter_C|SetVehicle _asbp_player_character 0)
  (Utilities|FlowControl|Gate true ; enters at Close
    (:Exit
      (Pawn|Possess (Game|GetPlayerController 0)))))

(fn ConstructionScript)